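; Keypad-locked sliding door that opens when the correct code is entered and closes on a wrong one.
; On BeginPlay it binds to the code-entered event of its KeyPad_UI widget, and CheckCode compares entries to CorrectCode, setting IsOpen and clearing the input.
; While IsOpen is true, the player's overlaps open and close the door automatically.
; A timeline slides the door's relative location, reversing to close.
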(event OnComponentBeginOverlap(Trigger)
  (params (OverlappedComponent :type Primitive%20Component%20Object%20Reference) (OtherActor :type Actor%20Object%20Reference) (OtherComp :type Primitive%20Component%20Object%20Reference) (OtherBodyIndex :type Integer) (bFromSweep :type Boolean) (SweepResult :type Hit%20Result%20Structure%20%28by%20ref%29))
  (if (== OtherActor (Game|GetPlayerCharacter 0))
    (if (Variables|Default|GetisOpen)
      (CallFunction|OpenDoor))))

(event Custom|OpenDoor
  (Variables|Default|SetisOpen true)
  (bind _doorsliding (Timeline|Timeline_0 Play)
    (:Update
      (Transformation|SetRelativeLocation (Variables|Default|GetDoor) _doorsliding false false))))

(event Custom|CloseDoor
  (bind _doorsliding (Timeline|Timeline_0 Reverse)
    (:Update
      (Transformation|SetRelativeLocation (Variables|Default|GetDoor) _doorsliding false false))))

(event Collision|EventActorEndOverlap
  (params (OtherActor :type Actor%20Object%20Reference))
  (if (== (Game|GetPlayerCharacter 0) OtherActor)
    (if (Variables|Default|GetisOpen)
      (CallFunction|CloseDoor))))

(event EventBeginPlay
  (bind _askey_pad_ui (Utilities|Casting|CastToKeyPad_UI (UserInterface|GetUserWidgetObject (Variables|Default|GetKeypadWidget))))
  (bind _output_get (Variables|Default|SetKeyPad_UI _askey_pad_ui))
  (EventDispatchers|BindEventtoCodeEntered _output_get (EventDispatchers|CreateEvent :!event CheckCode)))

(fn ConstructionScript)

(fn CheckCode
  (params (CodeEntered :type String) (KeyPad_UI :type Key%20Pad%20UI%20Object%20Reference))
  (if (Utilities|Enum|Equal(Enum) CodeEntered (Variables|Default|GetCorrectCode))
    (Variables|Default|SetisOpen true)
    (CallFunction|OpenDoor)
    (Variables|/Game/BlockBreaker/Blueprints/KeyPad_UI.KeyPad_UI_C|SetCurrentCode (Variables|Default|GetKeyPad_UI) "")
    (else
      (CallFunction|CloseDoor)
      (Variables|/Game/BlockBreaker/Blueprints/KeyPad_UI.KeyPad_UI_C|SetCurrentCode (Variables|Default|GetKeyPad_UI) "")
      (Variables|Default|SetisOpen false))))