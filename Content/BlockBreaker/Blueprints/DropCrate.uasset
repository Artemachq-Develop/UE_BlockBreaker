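; DropCrate is a damageable crate actor in BlockBreaker that drops a HealObject when its health runs out.
; AnyDamage passes damage to TakeDamage, which subtracts it from Health and clamps the result to a zero-to-one range.
; At zero, it hides the Sphere component, disables its collision and spawns the HealObject above the crate's location, leaving the actor itself in place.
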(event EventBeginPlay)

(event Collision|EventActorBeginOverlap
  (params (OtherActor :type Actor%20Object%20Reference)))

(event EventTick
  (params (DeltaSeconds :type Float%20%28single-precision%29)))

(event Game|Damage|EventAnyDamage
  (params (Damage :type Float%20%28single-precision%29) (DamageType :type Damage%20Type%20Object%20Reference) (InstigatedBy :type Controller%20Object%20Reference) (DamageCauser :type Actor%20Object%20Reference))
  (CallFunction|TakeDamage Damage))

(fn ConstructionScript)

(fn TakeDamage
  (params (Damage :type Float%20%28single-precision%29))
  (bind _sphere (Variables|Default|GetSphere))
  (bind _output_get (Variables|Default|SetHealth (Math|Float|Clamp(Float) (- (Variables|Default|GetHealth) Damage))))
  (if (== _output_get 0.0)
    (Rendering|SetVisibility _sphere false false)
    (Collision|SetCollisionEnabled _sphere "NoCollision")
    (Game|SpawnActorfromClass "/Game/BlockBreaker/Blueprints/HealObject.HealObject_C" (Math|Transform|MakeTransform (- (Transformation|GetActorLocation) "0,0.000000,-100.000000") "0, 0, 0" "1,1,1") "Undefined" 0 0)))