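; BP_Follower is a companion pawn that spins in place until the player touches it, then follows the flying player; it can also start active.
; On activation it registers with the player and starts two looping timers.
; One timer rerolls a random offset.
; The other queries the player, interpolating rotation to theirs and FloatingPawnMovement velocity toward the nearer left or right point plus offset, at a player-speed-based rate.
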(event OnComponentBeginOverlap(Box)
  (params (OverlappedComponent :type Primitive%20Component%20Object%20Reference) (OtherActor :type Actor%20Object%20Reference) (OtherComp :type Primitive%20Component%20Object%20Reference) (OtherBodyIndex :type Integer) (bFromSweep :type Boolean) (SweepResult :type Hit%20Result%20Structure%20%28by%20ref%29))
  (Utilities|Casting|CastToBP_Player OtherActor)
  (Variables|Default|SetcanMove true)
  (bind _output_get (Variables|Base|SetPlayer (Game|GetPlayerCharacter 0)))
  (Utilities|IsValid _output_get
    (:Is%20Valid
      (Class|BPIFollowerTalk|AddFollower(Message) _output_get self)
      (bind _returnvalue (Utilities|Time|SetTimerbyEvent (delegate Custom|GenerateRandomOffsetTick) (Variables|Default|GetRandomOffsetTime) true))
      (Variables|Default|SetRandomOffsetTimer _returnvalue)
      (bind _returnvalue_2 (Utilities|Time|SetTimerbyEvent (delegate Custom|VelocityUpdateTick) (Variables|Default|GetVelocityUpdateTime) true))
      (Variables|Default|SetVelocityUpdateTimer _returnvalue_2))))

(event Custom|VelocityUpdateTick
  (bind _floatingpawnmovement (Variables|Default|GetFloatingPawnMovement))
  (bind (_rot _left _right _speed) (Class|BPIFollowerTalk|FlyingPlayerQuery(Message) (Variables|Base|GetPlayer)))
  (Utilities|FlowControl|Sequence
    (:then_0
      (Transformation|SetActorRotation (Math|Interpolation|RInterpTo (Transformation|GetActorRotation) _rot (Variables|Default|GetVelocityUpdateTime) (Variables|Default|GetRinterpSpeed))))
    (:then_1
      (Variables|/Script/Engine.MovementComponent|SetVelocity _floatingpawnmovement (Math|Interpolation|VInterpTo (Variables|/Script/Engine.MovementComponent|GetVelocity _floatingpawnmovement) (* (Math|Vector|Normalize (- (+ (select (CallFunction|GetLR _left _right) _right _left) (Variables|Default|GetRandomOffset)) (Transformation|GetActorLocation))) (Math|Float|SelectFloat 1e+02 (+ (* _speed 0.9) 1.5e+02) (< (+ (* _speed 0.9) 1.5e+02) 2e+02))) (Variables|Default|GetVelocityUpdateTime) (Variables|Default|GetVinterpSpeed))))))

(event Custom|GenerateRandomOffsetTick
  (Variables|Default|SetRandomOffset (CallFunction|GenerateRandomOffset)))

(event EventBeginPlay
  (if (Variables|Default|GetcanMove)
    (bind _output_get (Variables|Base|SetPlayer (Game|GetPlayerCharacter 0)))
    (Utilities|IsValid _output_get
      (:Is%20Valid
        (Class|BPIFollowerTalk|AddFollower(Message) _output_get self)
        (bind _returnvalue (Utilities|Time|SetTimerbyEvent (delegate Custom|GenerateRandomOffsetTick) (Variables|Default|GetRandomOffsetTime) true))
        (Variables|Default|SetRandomOffsetTimer _returnvalue)
        (bind _returnvalue_2 (Utilities|Time|SetTimerbyEvent (delegate Custom|VelocityUpdateTick) (Variables|Default|GetVelocityUpdateTime) true))
        (Variables|Default|SetVelocityUpdateTimer _returnvalue_2)))))

(event EventCommandFollower
  (params (New%20Mode :type E_FlyingMode%20Enum :default "NewEnumerator0")))

(event EventTick
  (params (DeltaSeconds :type Float%20%28single-precision%29))
  (if (not (Variables|Default|GetcanMove))
    (Transformation|AddActorLocalRotation self (Math|Rotator|MakeRotator 0.0 (* (Variables|Default|GetRotation) DeltaSeconds) 0.0) false false)))

(fn ConstructionScript)

(fn GenerateRandomOffset
  (bind _randomoffsetminmax (Variables|Default|GetRandomOffsetMinMax))
  (return (Math|Vector|MakeVector (Math|Random|RandomFloatinRange (* -1 (.x _randomoffsetminmax)) (.x _randomoffsetminmax)) (Math|Random|RandomFloatinRange (* -1 (.y _randomoffsetminmax)) 0.0) (Math|Random|RandomFloatinRange (* -1 (.z _randomoffsetminmax)) 0.0))))

(fn GetLR
  (params (Left :type Vector) (Right :type Vector))
  (bind _returnvalue (Transformation|GetActorLocation))
  (return (> (Math|Vector|VectorLength (- _returnvalue Left)) (Math|Vector|VectorLength (- _returnvalue Right)))))

(fn FlyingPlayerQuery
  (return "0, 0, 0" "0, 0, 0" "0, 0, 0" 0.0))